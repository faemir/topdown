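; Enemy spawner actor that creates homing (EnemyB) and dumb (EnemyA) enemies at its own transform.
; A looping one-second timer calls SpawnEnemy, which spawns while its count is under 50.
; Both actor queries target EnemyA, so that count doubles EnemyA and ignores EnemyB.
; EnemyType selects the class and is re-rolled after each spawn, giving subsequent spawns a one-in-four chance of homing.
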(event `self.ReceiveBeginPlay`
  (`KismetSystemLibrary.K2_SetTimer` null "spawnEnemy" 1.0 true))

(fn `spawnEnemy`
  (bind _outactors (`GameplayStatics.GetAllActorsOfClass` "/Game/Blueprints/enemyA.enemyA_C"))
  (bind _outactors_2 (`GameplayStatics.GetAllActorsOfClass` "/Game/Blueprints/enemyA.enemyA_C"))
  (set `self.spawnCount` (+ (`KismetArrayLibrary.Array_Length` _outactors_2) (`KismetArrayLibrary.Array_Length` _outactors)))
  (if (< (`self.spawnCount`) 50)
    (if (== (`self.enemyType`) 0)
      ;[1 1 1] spawn homing enemy
      (`|SpawnActorFromClass` "/Game/Blueprints/enemyB.enemyB_C" (`self.GetTransform`))
      (set `self.enemyType` (`KismetMathLibrary.RandomIntegerInRange` 0 3))
      (else
        ;[1 1 1] spawn dumb enemy
        (`|SpawnActorFromClass` "/Game/Blueprints/enemyA.enemyA_C" (`self.GetTransform`))
        (set `self.enemyType` (`KismetMathLibrary.RandomIntegerInRange` 0 3))))))

(fn `UserConstructionScript`)