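; Enemy B is an enemy actor that flies constantly forward and periodically snaps to face the player ship, using a looping timer for simple homing.
; LaserBeam hits reduce Health; at zero it stops moving, awards score through the player controller and shatters its Destructible with radius damage.
; After a delay, a timeline toggles the debris visibility before destroying the actor.
; The construction script rolls random X/Y values through NewGoal, which nothing shown here reads.
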(event `self.ReceiveTick`
  (params (DeltaSeconds :type "Float (single-precision)"))
  ;[1 1 1] move forwards
  (if (<= (`self.health`) 0)
    (`self.K2_SetActorLocation` (`self.K2_GetActorLocation`))
    (else
      (`self.K2_SetActorLocation` (+ (`self.K2_GetActorLocation`) (* (`self.GetActorForwardVector`) 7.0))))))

(event `newHomingRot`
  ;[1 1 1] rotate facing the player
  (bind _asblueprint_player_ship_default_pawn (cast `/Game/Blueprints/Blueprint_PlayerShip_DefaultPawn` (`GameplayStatics.GetPlayerPawn` 0)))
  (`self.SetActorRotation` (`KismetMathLibrary.FindLookAtRotation` (`self.K2_GetActorLocation`) (`self.K2_GetActorLocation` _asblueprint_player_ship_default_pawn))))

(event `self.ReceiveBeginPlay`
  ;[1 1 1] rotate the enemy every few seconds
  (`KismetSystemLibrary.K2_SetTimer` null "newHomingRot" 3.0 true))

(event `self.ReceiveHit`
  (params (MyComp :type "PrimitiveComponent Object Reference") (Other :type "Actor Object Reference") (OtherComp :type "PrimitiveComponent Object Reference") (bSelfMoved :type Boolean) (HitLocation :type "Object.Vector Structure") (HitNormal :type "Object.Vector Structure") (NormalImpulse :type "Object.Vector Structure") (Hit :type "EngineTypes.HitResult Structure (by ref)"))
  ;[1 1 1] collision with weapon
  (if (== (`GameplayStatics.GetObjectClass` Other) "/Game/Blueprints/laserBeam.laserBeam_C")
    (set `self.health` (- (`self.health`) 5))
    (if (<= (`self.health`) 0)
      (bind _asnew_player_controller (cast `/Game/Blueprints/newPlayerController` (`GameplayStatics.GetPlayerController` 0)))
      (`/Game/Blueprints/newPlayerController.addScore` _asnew_player_controller (`self.scoreVal`))
      (`DestructibleComponent.ApplyRadiusDamage` (`self.Destructible`) 5.0 HitLocation 500.0 5000.0 true)
      (`KismetSystemLibrary.Delay` 2.0)
      (`Timeline|Timeline_0` :!via `PlayFromStart`
        (:`Finished`
          (`self.K2_DestroyActor`))
        (:`Toggle Vis`
          (`SceneComponent.ToggleVisibility` (`self.Destructible`) false))))))

(fn `newGoal`
  ;[1 1 1] new actor location target
  (set `self.ranY` (`KismetMathLibrary.RandomFloatInRange` -5.0 5.0))
  (set `self.ranX` (`KismetMathLibrary.RandomFloatInRange` -5.0 5.0)))

(fn `UserConstructionScript`
  (`self.newGoal`))