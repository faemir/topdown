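; Player ship pawn that moves along control-rotation axes and fires lasers with the gamepad's right stick.
; Right-stick input past a dead zone on either axis sets a target angle and spawns an offset LaserBeam, rate-limited by a delayed CanFire flag.
; Tick smoothly interpolates the ship's rotation toward that angle.
; BeginPlay activates the pawn's camera and makes it the player's view target.
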(event `InputAxisKey|Gamepad_RightX`
  (params (AxisValue :type "Float (single-precision)"))
  ;[1 1 1] pad stick rotation firing
  (if (or (> AxisValue 0.5) (< AxisValue -0.5))
    (set `self.rotateAngle` (`KismetMathLibrary.Conv_VectorToRotator` (`KismetMathLibrary.MakeVector` AxisValue (stale `InputAxisKey|Gamepad_RightY` AxisValue))) :!label _label)
    (if (`self.canFire`)
      (bind _returnvalue (`KismetMathLibrary.Conv_VectorToRotator` (`KismetMathLibrary.MakeVector` AxisValue (stale `InputAxisKey|Gamepad_RightY` AxisValue))))
      (`|SpawnActorFromClass` "/Game/Blueprints/laserBeam.laserBeam_C" (`KismetMathLibrary.MakeTransform` (+ (`self.K2_GetActorLocation`) (`KismetMathLibrary.GreaterGreater_VectorRotator` (`self.gun Offset`) _returnvalue)) _returnvalue))
      (set `self.canFire` false)
      (`KismetSystemLibrary.Delay` 0.2)
      (set `self.canFire` true))))

(event `InputAxisKey|Gamepad_RightY`
  (params (AxisValue :type "Float (single-precision)"))
  ;[1 1 1] pad stick rotation firing
  (if (or (> AxisValue 0.5) (< AxisValue -0.5))
    (goto _label)))

(event `self.ReceiveTick`
  (params (DeltaSeconds :type "Float (single-precision)"))
  ;[1 1 1] ship lerp rotation
  (`self.SetActorRotation` (`KismetMathLibrary.RInterpTo` (`self.K2_GetActorRotation`) (`self.rotateAngle`) DeltaSeconds (`self.rotateSpeed`))))

(event `InputAxis|MoveForward`
  (params (AxisValue :type "Float (single-precision)"))
  ;[1 1 1] ship movement
  (`self.AddMovementInput` (`KismetMathLibrary.GetForwardVector` (`self.GetControlRotation`)) AxisValue))

(event `self.ReceiveBeginPlay`
  ;[1 1 1] activate camera
  (`ActorComponent.SetActive` (`self.playercam`) true false)
  (`PlayerController.SetViewTargetWithBlend` (`GameplayStatics.GetPlayerController` 0) self 0.0 "VTBlend_Linear" 0.0 false))

(event `InputAxis|MoveRight`
  (params (AxisValue :type "Float (single-precision)"))
  ;[1 1 1] ship movement
  (`self.AddMovementInput` (`KismetMathLibrary.GetRightVector` (`self.GetControlRotation`)) AxisValue))

(fn `UserConstructionScript`)