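; Enemy actor that drifts around at random and awards score to the player when destroyed by laser fire.
; Tick moves it in X and Y by a random per-frame offset without sweep, which NewGoal sets at construction and re-rolls about every 4 seconds through a Delay.
; LaserBeam hits reduce Health; at zero it adds ScoreVal through newPlayerController and destroys itself.
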(event `self.ReceiveTick`
  (params (DeltaSeconds :type "Float (single-precision)"))
  ;[1 1 1] random movement
  (`self.K2_SetActorLocation` (`KismetMathLibrary.MakeVector` (+ (.x (`self.K2_GetActorLocation`)) (`self.ranY`)) (+ (.y (`self.K2_GetActorLocation`)) (`self.ranX`)) (.z (`self.K2_GetActorLocation`))))
  (set `self.newLoc` true)
  (if (`self.newLoc`)
    (`KismetSystemLibrary.Delay` 4.0)
    (set `self.newLoc` true)
    (`self.newGoal`)))

(event `self.ReceiveHit`
  (params (MyComp :type "PrimitiveComponent Object Reference") (Other :type "Actor Object Reference") (OtherComp :type "PrimitiveComponent Object Reference") (bSelfMoved :type Boolean) (HitLocation :type "Object.Vector Structure") (HitNormal :type "Object.Vector Structure") (NormalImpulse :type "Object.Vector Structure") (Hit :type "EngineTypes.HitResult Structure (by ref)"))
  ;[1 1 1] collision with weapon
  (if (== (`GameplayStatics.GetObjectClass` Other) "/Game/Blueprints/laserBeam.laserBeam_C")
    (set `self.health` (- (`self.health`) 5))
    (if (<= (`self.health`) 0)
      (bind _asnewplayercontroller_c (cast `/Game/Blueprints/newPlayerController` (`GameplayStatics.GetPlayerController` 0)))
      (`/Game/Blueprints/newPlayerController.addScore` _asnewplayercontroller_c (`self.scoreVal`))
      (`self.K2_DestroyActor`))))

(fn `newGoal`
  ;[1 1 1] new actor location target
  (set `self.ranY` (`KismetMathLibrary.RandomFloatInRange` -5.0 5.0))
  (set `self.ranX` (`KismetMathLibrary.RandomFloatInRange` -5.0 5.0)))

(fn `UserConstructionScript`
  (`self.newGoal`))